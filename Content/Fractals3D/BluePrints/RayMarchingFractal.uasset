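; Actor that renders a ray-marched 3D fractal on its static mesh through a material instance that follows the actor's transform.
; The Construction Script applies the material and pushes rotation axes, X-based scale and location as parameters for editor preview.
; BeginPlay creates a dynamic instance, and Tick updates those transform parameters plus an accumulated Time scaled by TimerMult to animate it.
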(event `self.ReceiveBeginPlay`
  (bind _returnvalue (`KismetMaterialLibrary.CreateDynamicMaterialInstance` (`self.MatInstance`)))
  (bind _output_get (set `self.DynamicMat` _returnvalue))
  (`PrimitiveComponent.SetMaterial` (`self.StaticMeshComponent`) 0 _output_get))

(event `self.ReceiveTick`
  (params (DeltaSeconds :type "Float (single-precision)"))
  (bind _dynamicmat (`self.DynamicMat`))
  (bind (_x _y _z) (`KismetMathLibrary.BreakRotIntoAxes` (`self.K2_GetActorRotation`)))
  (bind _output_get (set `self.Seconds` (+ (`self.Seconds`) (* DeltaSeconds (`self.TimerMult`)))))
  (`MaterialInstanceDynamic.SetScalarParameterValue` _dynamicmat "Time" _output_get)
  (`MaterialInstanceDynamic.SetVectorParameterValue` _dynamicmat "RotMatRow1" (make `LinearColor` (.x _x) (.y _x) (.z _x) 1.0))
  (`MaterialInstanceDynamic.SetVectorParameterValue` _dynamicmat "RotMatRow2" (make `LinearColor` (.x _y) (.y _y) (.z _y) 1.0))
  (`MaterialInstanceDynamic.SetVectorParameterValue` _dynamicmat "RotMatRow3" (make `LinearColor` (.x _z) (.y _z) (.z _z) 1.0))
  (`MaterialInstanceDynamic.SetScalarParameterValue` _dynamicmat "ObjectScale" (* (`KismetMathLibrary.Abs` (.x (`self.GetActorScale3D`))) (`self.ScaleKoeff`)))
  (`MaterialInstanceDynamic.SetVectorParameterValue` _dynamicmat "ObjectPosition" (make `LinearColor` (.x (`self.K2_GetActorLocation`)) (.y (`self.K2_GetActorLocation`)) (.z (`self.K2_GetActorLocation`)) 1.0)))

(fn `UserConstructionScript`
  (bind _staticmeshcomponent (`self.StaticMeshComponent`))
  (bind (_x _y _z) (`KismetMathLibrary.BreakRotIntoAxes` (`self.K2_GetActorRotation`)))
  (`PrimitiveComponent.SetMaterial` _staticmeshcomponent 0 (`self.MatInstance`))
  (`MeshComponent.SetVectorParameterValueOnMaterials` _staticmeshcomponent "RotMatRow1" (`KismetMathLibrary.MakeVector` (.x _x) (.y _x) (.z _x)))
  (`MeshComponent.SetVectorParameterValueOnMaterials` _staticmeshcomponent "RotMatRow2" (`KismetMathLibrary.MakeVector` (.x _y) (.y _y) (.z _y)))
  (`MeshComponent.SetVectorParameterValueOnMaterials` _staticmeshcomponent "RotMatRow3" (`KismetMathLibrary.MakeVector` (.x _z) (.y _z) (.z _z)))
  (`MeshComponent.SetScalarParameterValueOnMaterials` _staticmeshcomponent "ObjectScale" (* (`KismetMathLibrary.Abs` (.x (`self.GetActorScale3D`))) (`self.ScaleKoeff`)))
  (`MeshComponent.SetVectorParameterValueOnMaterials` _staticmeshcomponent "ObjectPosition" (`KismetMathLibrary.MakeVector` (.x (`self.K2_GetActorLocation`)) (.y (`self.K2_GetActorLocation`)) (.z (`self.K2_GetActorLocation`)))))