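; Audio-reactive ray-marched fractal Blueprint that plays audio on BeginPlay and drives a dynamic material from precomputed sound analysis every tick.
; UpdateAudio averages a range of Constant-Q bands to blend two colors, the second weighted by loudness, into GradientColorHigh.
; Loudness also lowers the material's Scale parameter and raises Loop0 above a threshold.
; Analysis is sampled at game time rather than the audio component's playback position.
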(event `self.ReceiveBeginPlay`
  (`parent.ReceiveBeginPlay`)
  (`AudioComponent.Play` (`self.Audio`) 0.0))

(event `self.ReceiveTick`
  (params (DeltaSeconds :type "Float (single-precision)"))
  (`parent.ReceiveTick` DeltaSeconds)
  (`self.UpdateAudio`))

(fn `UpdateAudio`
  (bind _dynamicmat (`self.DynamicMat`))
  (bind _outloudness (`LoudnessNRT.GetNormalizedLoudnessAtTime` (`self.Loudness`) (`KismetSystemLibrary.GetGameTimeInSeconds`)))
  (set `self.Sum` 0.0)
  (for _index (range (`self.Begin`) (+ (`self.End`) 1))
    (set `self.Sum` (+ (`self.Sum`) (`|GetArrayItem` (`ConstantQNRT.GetNormalizedChannelConstantQAtTime` (`self.Freq`) (`KismetSystemLibrary.GetGameTimeInSeconds`) 0) _index))))
  (bind _output_get (set `self.Sum` (/ (`self.Sum`) (- (`self.End`) (`self.Begin`) -1))))
  (`MaterialInstanceDynamic.SetScalarParameterValue` _dynamicmat "Scale" (+ (* _outloudness 0.5 -1.0) 1.6))
  (`MaterialInstanceDynamic.SetVectorParameterValue` _dynamicmat "GradientColorHigh" (make `LinearColor` (.x (+ (* (`self.Color`) _output_get) (* (- 1.0 _output_get) (`self.Color2`) _outloudness))) (.y (+ (* (`self.Color`) _output_get) (* (- 1.0 _output_get) (`self.Color2`) _outloudness))) (.z (+ (* (`self.Color`) _output_get) (* (- 1.0 _output_get) (`self.Color2`) _outloudness)))))
  (set `self.Loop_0` (+ 1.0 (/ (`KismetMathLibrary.Abs` (`KismetMathLibrary.FClamp` (- _outloudness 0.75))) 0.05))))

(fn `UserConstructionScript`
  (`parent.UserConstructionScript`))